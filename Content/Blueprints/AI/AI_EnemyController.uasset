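; AI controller for enemy characters that connects AI perception to the AI_EnemyBT behavior tree.
; On possess, it caches the AI_EnemyCharacter pawn and starts the tree.
; Perception updates of MY_CHARACTER_CONTROLLER actors write sensing success to the CanSee blackboard key, with debug prints.
; Walk and Run events forward to the enemy, and an L key binding calls its Ragdoll.
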(event OnTargetPerceptionUpdated(AIPerception)
  (params (Actor :type Actor%20Object%20Reference) (Stimulus :type AI%20Stimulus%20Structure))
  (Utilities|Casting|CastToMY_CHARACTER_CONTROLLER Actor
    (:then
      (AI|Components|Blackboard|SetValueasBool (AI|GetBlackboard 0) (Utilities|Name|MakeLiteralName "CanSee") (.bSuccessfullySensed (Utilities|Struct|BreakAIStimulus Stimulus)))
      (Development|PrintString "Seen"))
    (:CastFailed
      (Development|PrintString "UnSeen"))))

(event Custom|Walk
  (Default|Walk (Variables|Default|GetEnemy)))

(event Custom|Run
  (Default|Run (Variables|Default|GetEnemy)))

(event EventPossess
  (params (PossessedPawn :type Pawn%20Object%20Reference))
  (bind _asai_enemy_character (Utilities|Casting|CastToAI_EnemyCharacter PossessedPawn))
  (Variables|Default|SetEnemy _asai_enemy_character)
  (AI|RunBehaviorTree "/Game/Blueprints/AI/AI_EnemyBT.AI_EnemyBT"))

(event Input|KeyboardEvents|L
  (params (Key :type Key%20Structure :default "None"))
  (:Pressed
    (Default|Ragdoll (Variables|Default|GetEnemy))))

(fn ConstructionScript)