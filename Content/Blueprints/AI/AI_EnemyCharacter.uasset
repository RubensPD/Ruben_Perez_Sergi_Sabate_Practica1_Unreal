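; AI enemy character Blueprint that ragdolls itself on a fixed timer after spawning.
; BeginPlay allows walking, then after a delay sets the death flag, disables movement and turns on full mesh physics, blended from the pelvis down.
; Walk and Run events switch max walk speed.
; A Death function simulates capsule and bone physics but is uncalled here, and the Ragdoll event actually switches simulation off below the pelvis.
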(event Custom|Walk
  (Variables|/Script/Engine.CharacterMovementComponent|SetMaxWalkSpeed (Variables|Character|GetCharacterMovement) 1.5e+02))

(event Custom|Run
  (Variables|/Script/Engine.CharacterMovementComponent|SetMaxWalkSpeed (Variables|Character|GetCharacterMovement) 4e+02))

(event Custom|Ragdoll
  (bind _returnvalue (Utilities|Name|MakeLiteralName "pelvis"))
  (bind _mesh (Variables|Character|GetMesh))
  (Class|SkeletalMeshComponent|SetAllBodiesBelowSimulatePhysics _mesh _returnvalue false true)
  (Class|SkeletalMeshComponent|SetAllBodiesBelowPhysicsBlendWeight _mesh _returnvalue 1.0 false true))

(event EventBeginPlay
  (Variables|Default|SetcanWalk true)
  (Utilities|FlowControl|Delay 8.0)
  (Variables|Default|SetActivateDeath true)
  (Variables|Default|SetcanWalk false)
  (if (not false)
    (Pawn|Components|CharacterMovement|DisableMovement (Variables|Character|GetCharacterMovement))
    (Collision|SetCollisionEnabled (Variables|Character|GetMesh) "QueryAndPhysics")
    (Class|SkeletalMeshComponent|SetAllBodiesSimulatePhysics (Variables|Character|GetMesh) true)
    (Class|SkeletalMeshComponent|SetAllBodiesBelowPhysicsBlendWeight (Variables|Character|GetMesh) (Utilities|Name|MakeLiteralName "pelvis") 1.0 true true)))

(fn ConstructionScript)

(fn Death
  (bind _capsulecomponent (Variables|Collision|GetCapsuleComponent))
  (bind _mesh (Variables|Character|GetMesh))
  (Physics|SetSimulatePhysics _capsulecomponent true)
  (Collision|SetCollisionResponsetoChannel _capsulecomponent "ECC_PhysicsBody" "ECR_Overlap")
  (Class|SkeletalMeshComponent|SetAllBodiesBelowSimulatePhysics _mesh (Class|SkinnedMeshComponent|GetBoneName _mesh 1) true true))